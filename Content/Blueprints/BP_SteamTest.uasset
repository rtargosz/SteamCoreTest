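; BP_SteamTest is a Steam integration smoke test that runs on BeginPlay and reports results through PrintString.
; If Steam is available, it prints the Steam ID, App ID and achievement count, then asynchronously looks up the TOTAL_MONSTERS_KILLED leaderboard.
; It also sends a vote-ranked Workshop UGC query, whose callback event stores the query handle and prints the result count or failure.
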(event Custom|CustomEvent
  (params (Data :type Steam%20UGC%20Query%20Completed%20Structure%20%28by%20ref%29) (bWasSuccessful :type Boolean))
  (bind (_handle _result _numresultsreturned) (Utilities|Struct|BreakSteamUGCQueryCompleted Data))
  (if bWasSuccessful
    (Variables|Default|SetUGCQueryHandle _handle)
    (Development|PrintString (Utilities|String|Append "NumResults: " (Utilities|String|ToString(Integer) _numresultsreturned)) true true "(R=0.132069,G=1.000000,B=0.000000,A=1.000000)" 3e+01)
    (else
      (Development|PrintString (Utilities|String|Append "Send Query UGC Request Failed: " (Utilities|String|EnumtoString _result)) true true "(R=1.000000,G=0.036562,B=0.000000,A=1.000000)" 3e+01))))

(event EventBeginPlay
  (bind _returnvalue (Class|Utils|GetAppIDPure))
  (if (Class|SteamUtilities|IsSteamAvailable)
    (Utilities|FlowControl|Sequence
      (:then_0
        (Development|PrintString (Utilities|String|Append "SteamID: " (Class|SteamUtilities|BreakSteamID (Class|User|GetSteamIDPure))) true true "(R=0.000000,G=0.430443,B=1.000000,A=1.000000)" 3e+01)
        (Development|PrintString (Utilities|String|Append "Steam AppID: " (Utilities|String|ToString(Integer) (Class|Utils|GetAppIDPure))) true true "(R=0.000000,G=0.430443,B=1.000000,A=1.000000)" 3e+01)
        (bind _returnvalue_2 (Class|UserStats|GetNumAchievements))
        (Development|PrintString (Utilities|String|Append "NumAchievements" (Utilities|String|ToString(Integer) _returnvalue_2)) true true "(R=0.000000,G=0.430443,B=1.000000,A=1.000000)" 3e+01)
        (bind (_data _bwassuccessful) (|FindLeaderboardAsync "TOTAL_MONSTERS_KILLED" 1e+01)
          (:OnCallback
            (if _bwassuccessful
              (if (.bLeaderboardFound (Utilities|Struct|BreakLeaderboardFindResult _data))
                (Development|PrintString (Utilities|String|Append "Leaderboard found: " "TOTAL_MONSTERS_KILLED") true true "(R=0.000000,G=0.430443,B=1.000000,A=1.000000)" 3e+01))))))
      (:then_1
        (bind _returnvalue_3 (Class|UGC|CreateQueryAllUGCRequest "RankedByVote" "Items" _returnvalue _returnvalue 1))
        (Class|UGC|SendQueryUGCRequest (Subsystems|GetUGC) (delegate Custom|CustomEvent) _returnvalue_3)
        (Development|PrintString "Send Query UGCRequest" true true "(R=0.000000,G=0.430443,B=1.000000,A=1.000000)" 3e+01)))
    (else
      (Development|PrintString "Steam Not Available" true true "(R=1.000000,G=0.036562,B=0.000000,A=1.000000)" 3e+01))))

(fn ConstructionScript)